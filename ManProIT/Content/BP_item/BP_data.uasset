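; BP_data is a data item actor whose look reflects the type, target IP address and ID it receives on spawn.
; SetOnSpawn stores the data and pickability, then calls ShowByData, which reveals the music mesh and colors it by IP; other types show nothing.
; Nested ID checks govern scaling and a switch to Vehicle collision for non-pickable items.
; PickUp and destroy are empty stubs, and the held-item check is unconnected.
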(event Custom|SetOnSpawn
  (params (data%20value :type Struct%20Data%20Value%20Structure) (canBePicked :type Boolean))
  (Variables|Default|Setcan%20be%20picked canBePicked)
  (bind _output_get (Variables|Default|Setdata%20value data%20value))
  (CallFunction|ShowbyData (Utilities|Array|Get(acopy) (.0id10isvirus>0isScoreValuenotvirus (Utilities|Struct|BreakStruct_dataValue _output_get))) (.Datatype (Utilities|Struct|BreakStruct_dataValue _output_get)) (.IPaddressTarget (Utilities|Struct|BreakStruct_dataValue _output_get))))

(event Custom|PickUp)

(event Custom|destroy)

(event EventBeginPlay)

(event Collision|EventActorBeginOverlap
  (params (OtherActor :type Actor%20Object%20Reference)))

(event EventTick
  (params (DeltaSeconds :type Float%20%28single-precision%29)))

(fn ConstructionScript)

(fn ShowbyData
  (params (dataID :type Integer) (Type :type Text) (IP :type Text))
  (bind _musicdata (Variables|Default|GetMusicData))
  (if (Utilities|Enum|Equal(Enum) Type (LocalVariables|GettypeMusic))
    (Rendering|SetVisibility _musicdata true true)
    (LocalVariables|SetDataUsed _musicdata)
    (if (Utilities|Enum|Equal(Enum) IP (LocalVariables|Getip1))
      (Rendering|Material|SetMaterial (LocalVariables|GetDataUsed) 0 "/Game/FPWeapon/Materials/BaseMaterial.BaseMaterial")
      (if (< dataID 991) :!label _label
        (if (== dataID 991)
          (Transformation|SetWorldTransform (LocalVariables|GetDataUsed) (Math|Transform|MakeTransform (Transformation|GetWorldLocation (LocalVariables|GetDataUsed)) (Transformation|GetWorldRotation (LocalVariables|GetDataUsed)) "0.700000,0.700000,0.700000") false false)
          (if (not (Variables|Default|Getcan%20be%20picked)) :!label _label_2
            (Collision|SetCollisionObjectType (LocalVariables|GetDataUsed) "ECC_Vehicle"))
          (elif (not (== dataID 992))
            (if true
              (goto _label_2)))))
      (elif (Utilities|Enum|Equal(Enum) IP (LocalVariables|Getip2))
        (Rendering|Material|SetMaterial (LocalVariables|GetDataUsed) 0 "/Game/FPWeapon/Materials/FirstPersonProjectileMaterial.FirstPersonProjectileMaterial")
        (goto _label)
        (elif (Utilities|Enum|Equal(Enum) IP (LocalVariables|Getip3))
          (Rendering|Material|SetMaterial (LocalVariables|GetDataUsed) 0 "/Game/Asset/kuning.kuning")
          (goto _label)
          (elif (Utilities|Enum|Equal(Enum) IP (LocalVariables|Getip4))
            (Rendering|Material|SetMaterial (LocalVariables|GetDataUsed) 0 "/Game/LevelPrototyping/Materials/M_Solid.M_Solid")
            (goto _label)
            (elif (Utilities|Enum|Equal(Enum) IP (LocalVariables|Getip5))
              (Rendering|Material|SetMaterial (LocalVariables|GetDataUsed) 0 "/Game/LevelPrototyping/Materials/MI_Solid_Blue.MI_Solid_Blue")
              (goto _label)
              (elif (Utilities|Enum|Equal(Enum) IP (LocalVariables|Getip6))
                (Rendering|Material|SetMaterial (LocalVariables|GetDataUsed) 0 "/Game/Asset/SVGMat.SVGMat")
                (goto _label)))))))
    (elif false
      _)))