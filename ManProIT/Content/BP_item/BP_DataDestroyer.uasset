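; BP_DataDestroyer is an item Blueprint that runs a timed data-burning process.
; The processDataBurning event shows the Data component and starts a three-second countdown.
; A looping short Delay decrements TimeToBurn and writes the remaining value to a TextRender, without using Tick or a Timeline.
; When the countdown runs out, it hides Data and resets ItemID to zero.
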(event Custom|processDataBurning
  (Rendering|SetVisibility (Variables|Default|Getdata) true false)
  (Variables|Default|Settime%20to%20burn 3.0)
  (Utilities|FlowControl|Delay 0.01 :!label _label)
  (bind _output_get (Variables|Default|Settime%20to%20burn (- (Variables|Default|Gettime%20to%20burn) 0.01)))
  (Rendering|Components|TextRender|SetText (Variables|Default|GetTextRender) (Utilities|Text|ToText(Float) _output_get "HalfToEven"))
  (if (> _output_get 0.0)
    (goto _label)
    (else
      (Rendering|SetVisibility (Variables|Default|Getdata) false false)
      (Variables|Default|SetitemID 0))))

(event EventBeginPlay)

(event Collision|EventActorBeginOverlap
  (params (OtherActor :type Actor%20Object%20Reference)))

(event EventTick
  (params (DeltaSeconds :type Float%20%28single-precision%29)))

(fn ConstructionScript)