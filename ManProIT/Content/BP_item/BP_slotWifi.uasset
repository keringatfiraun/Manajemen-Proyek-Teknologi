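; BP_slotWifi is a wifi slot actor that keeps one BP_data item spawned at its own transform.
; After a random delay, it spawns the item flagged InWifi and not pickable, using a random entry from the player character's inventory StructData.
; DataTaken polls every two seconds and restarts the spawn once the item is no longer valid.
; Take returns the current item without clearing it.
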(event Custom|spawnData
  (bind _returnvalue (Transformation|GetActorTransform))
  (Development|PrintString "Hello")
  (bind _asbp_first_person_character (Utilities|Casting|CastToBP_FirstPersonCharacter (Game|GetPlayerCharacter 0)))
  (Utilities|FlowControl|Delay (Math|Random|RandomFloatinRange 3.0 1e+01))
  (bind _returnvalue_2 (Game|SpawnActorfromClass "/Game/BP_item/BP_data.BP_data_C" (Math|Transform|MakeTransform (.location _returnvalue) (.rotation _returnvalue) (.scale _returnvalue)) "Undefined" 0 0))
  (Variables|/Game/BP_item/BP_data.BP_data_C|SetinWifi _returnvalue_2 true)
  (Default|SetonSpawn _returnvalue_2 (Utilities|Array|Get(acopy) (Variables|/Game/BP_item/WG_inventory.WG_inventory_C|GetStruct_data (Variables|/Game/FirstPerson/Blueprints/BP_FirstPersonCharacter.BP_FirstPersonCharacter_C|GetInventory _asbp_first_person_character)) (Math|Random|RandomIntegerinRange 0 (- (Utilities|Array|Length (Variables|/Game/BP_item/WG_inventory.WG_inventory_C|GetStruct_data (Variables|/Game/FirstPerson/Blueprints/BP_FirstPersonCharacter.BP_FirstPersonCharacter_C|GetInventory _asbp_first_person_character))) 1))) false)
  (Variables|Default|Setdata _returnvalue_2)
  (CallFunction|DataTaken))

(event Custom|DataTaken
  (Utilities|IsValid (Variables|Default|Getdata)
    (:Is%20Valid
      (Utilities|FlowControl|Delay 2.0)
      (CallFunction|DataTaken))
    (:Is%20Not%20Valid
      (CallFunction|SpawnData))))

(event EventBeginPlay
  (CallFunction|SpawnData))

(event Collision|EventActorBeginOverlap
  (params (OtherActor :type Actor%20Object%20Reference)))

(event EventTick
  (params (DeltaSeconds :type Float%20%28single-precision%29)))

(fn ConstructionScript)

(fn Take
  (return (Variables|Default|Getdata)))