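; Slot actor that processes a delivered data item, identified by ItemCode, as part of a scoring game.
; processData shows the matching data cube or virus mesh, runs a countdown on the TextRender through a looping Delay, then hides the cube.
; It looks the code up in the player's Inventory StructData: viruses or mismatched IP targets cost a life, matching ones add score.
; The inventory then updates and the slot's ItemCode clears.
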(event Custom|processData
  (if (!= (Variables|Default|GetItemCode) 0)
    (CallFunction|ShowCurrentData (Variables|Default|GetItemCode))
    (Variables|Default|SettimeUntilProccessed 3.0)
    (Utilities|FlowControl|Delay 0.01 :!label _label)
    (Variables|Default|SettimeUntilProccessed (- (Variables|Default|GettimeUntilProccessed) 0.01))
    (if (> (Variables|Default|GettimeUntilProccessed) 0.0)
      (Rendering|Components|TextRender|SetText (Variables|Default|GetTextRender) (Utilities|Text|ToText(Float) (Variables|Default|GettimeUntilProccessed) "HalfToEven"))
      (goto _label)
      (else
        (Rendering|SetVisibility (Variables|Default|GetCube) false false)
        (bind _asbp_first_person_character (Utilities|Casting|CastToBP_FirstPersonCharacter (Game|GetPlayerCharacter 0)))
        (bind _array_element (Utilities|Array|ForEachLoopwithBreak (Variables|/Game/BP_item/WG_inventory.WG_inventory_C|GetStruct_data (Variables|/Game/FirstPerson/Blueprints/BP_FirstPersonCharacter.BP_FirstPersonCharacter_C|GetInventory _asbp_first_person_character)))
          (:LoopBody
            (if (== (Variables|Default|GetItemCode) (Utilities|Array|Get(acopy) (.0id10isvirus>0isScoreValuenotvirus (Utilities|Struct|BreakStruct_dataValue _array_element))))
              (bind _asbp_first_person_character_2 (Utilities|Casting|CastToBP_FirstPersonCharacter (Game|GetPlayerCharacter 0)))
              (if (== (Utilities|Array|Get(acopy) (.0id10isvirus>0isScoreValuenotvirus (Utilities|Struct|BreakStruct_dataValue _array_element)) 1) 0)
                (Development|PrintString "termasuk virus")
                (Variables|/Game/BP_item/WG_inventory.WG_inventory_C|Setlives (Variables|/Game/FirstPerson/Blueprints/BP_FirstPersonCharacter.BP_FirstPersonCharacter_C|GetInventory _asbp_first_person_character_2) (- (Variables|/Game/BP_item/WG_inventory.WG_inventory_C|Getlives (Variables|/Game/FirstPerson/Blueprints/BP_FirstPersonCharacter.BP_FirstPersonCharacter_C|GetInventory _asbp_first_person_character_2)) 1) :!label _label_2)
                (elif (Utilities|Enum|Equal(Enum) (.IPaddressTarget (Utilities|Struct|BreakStruct_dataValue _array_element)) (Variables|Default|GetIP))
                  (Variables|/Game/BP_item/WG_inventory.WG_inventory_C|Setscore (Variables|/Game/FirstPerson/Blueprints/BP_FirstPersonCharacter.BP_FirstPersonCharacter_C|GetInventory _asbp_first_person_character_2) (+ (Variables|/Game/BP_item/WG_inventory.WG_inventory_C|Getscore (Variables|/Game/FirstPerson/Blueprints/BP_FirstPersonCharacter.BP_FirstPersonCharacter_C|GetInventory _asbp_first_person_character_2)) (Utilities|Array|Get(acopy) (.0id10isvirus>0isScoreValuenotvirus (Utilities|Struct|BreakStruct_dataValue _array_element)) 1)))
                  (else
                    (Development|PrintString "data ke ip salah")
                    (goto _label_2))))
              (Default|Update (Variables|/Game/FirstPerson/Blueprints/BP_FirstPersonCharacter.BP_FirstPersonCharacter_C|GetInventory _asbp_first_person_character_2))
              (Variables|Default|SetItemCode 0))))))
    (else
      (CallFunction|HideAllData))))

(event EventBeginPlay)

(event EventTick
  (params (DeltaSeconds :type Float%20%28single-precision%29)))

(fn ConstructionScript)

(fn ShowCurrentData
  (params (DataID :type Integer))
  (if (>= DataID 1)
    (if (<= DataID 6)
      (Rendering|SetVisibility (Variables|Default|GetCube) true true)
      (else
        (if (== DataID 991) :!label _label
          (Rendering|SetVisibility (Variables|Default|GetVirus) true true)
          (else
            (Development|PrintString "Error ID tidak di kenal")))))
    (else
      (goto _label))))

(fn HideAllData
  (Rendering|SetVisibility (Variables|Default|GetCube) false true)
  (Rendering|SetVisibility (Variables|Default|GetVirus) false true))