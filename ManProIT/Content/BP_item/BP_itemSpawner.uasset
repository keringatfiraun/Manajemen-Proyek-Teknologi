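; Item spawner that presents incoming data items, normal or virus, in waves by toggling Cube or Virus mesh visibility.
; After a random delay it picks an ID from the player inventory's StructData, retrying immediately when the target IP matches its own, though ID and IP use separate random rolls.
; IsTaken hides the meshes, increments the count and requeues until the count exceeds DataIncomingLimit.
; Older SpawnActor logic remains disconnected.
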(event Custom|queue%20data
  (bind _ip (Variables|Default|GetIP))
  (Utilities|FlowControl|Delay (Math|Random|RandomFloatinRange 3.0 1e+01))
  (bind _asbp_first_person_character (Utilities|Casting|CastToBP_FirstPersonCharacter (Game|GetPlayerCharacter 0)))
  (if (<= (Variables|Default|GetdataCount) (Variables|Default|GetdataIncomingLimit))
    (bind _output_get (Variables|Default|SetitemId (Utilities|Array|Get(acopy) (.0id10isvirus>0isScoreValuenotvirus (Utilities|Struct|BreakStruct_dataValue (Utilities|Array|Get(acopy) (Variables|/Game/BP_item/WG_inventory.WG_inventory_C|GetStruct_data (Variables|/Game/FirstPerson/Blueprints/BP_FirstPersonCharacter.BP_FirstPersonCharacter_C|GetInventory _asbp_first_person_character)) (Math|Random|RandomIntegerinRange 0 (- (Utilities|Array|Length (Variables|/Game/BP_item/WG_inventory.WG_inventory_C|GetStruct_data (Variables|/Game/FirstPerson/Blueprints/BP_FirstPersonCharacter.BP_FirstPersonCharacter_C|GetInventory _asbp_first_person_character))) 1))))))))
    (Development|PrintText _ip)
    (Development|PrintText (.IPaddressTarget (Utilities|Struct|BreakStruct_dataValue (Utilities|Array|Get(acopy) (Variables|/Game/BP_item/WG_inventory.WG_inventory_C|GetStruct_data (Variables|/Game/FirstPerson/Blueprints/BP_FirstPersonCharacter.BP_FirstPersonCharacter_C|GetInventory _asbp_first_person_character)) (Math|Random|RandomIntegerinRange 0 (- (Utilities|Array|Length (Variables|/Game/BP_item/WG_inventory.WG_inventory_C|GetStruct_data (Variables|/Game/FirstPerson/Blueprints/BP_FirstPersonCharacter.BP_FirstPersonCharacter_C|GetInventory _asbp_first_person_character))) 1))))))
    (if (Utilities|Enum|NotEqual(Enum) (.IPaddressTarget (Utilities|Struct|BreakStruct_dataValue (Utilities|Array|Get(acopy) (Variables|/Game/BP_item/WG_inventory.WG_inventory_C|GetStruct_data (Variables|/Game/FirstPerson/Blueprints/BP_FirstPersonCharacter.BP_FirstPersonCharacter_C|GetInventory _asbp_first_person_character)) (Math|Random|RandomIntegerinRange 0 (- (Utilities|Array|Length (Variables|/Game/BP_item/WG_inventory.WG_inventory_C|GetStruct_data (Variables|/Game/FirstPerson/Blueprints/BP_FirstPersonCharacter.BP_FirstPersonCharacter_C|GetInventory _asbp_first_person_character))) 1))))) _ip)
      (CallFunction|ShowCurrentData _output_get)
      (else
        (CallFunction|QueueWithoutDelay)))
    (else
      (Development|PrintString "wave selesai"))))

(event Custom|IsTaken
  (CallFunction|HideAllData)
  (Variables|Default|SetitemId 0)
  (Variables|Default|SetdataCount (+ (Variables|Default|GetdataCount) 1))
  (CallFunction|QueueData))

(event Custom|queue%20without%20delay
  (bind _ip (Variables|Default|GetIP))
  (bind _asbp_first_person_character (Utilities|Casting|CastToBP_FirstPersonCharacter (Game|GetPlayerCharacter 0)))
  (if (<= (Variables|Default|GetdataCount) (Variables|Default|GetdataIncomingLimit))
    (bind _output_get (Variables|Default|SetitemId (Utilities|Array|Get(acopy) (.0id10isvirus>0isScoreValuenotvirus (Utilities|Struct|BreakStruct_dataValue (Utilities|Array|Get(acopy) (Variables|/Game/BP_item/WG_inventory.WG_inventory_C|GetStruct_data (Variables|/Game/FirstPerson/Blueprints/BP_FirstPersonCharacter.BP_FirstPersonCharacter_C|GetInventory _asbp_first_person_character)) (Math|Random|RandomIntegerinRange 0 (- (Utilities|Array|Length (Variables|/Game/BP_item/WG_inventory.WG_inventory_C|GetStruct_data (Variables|/Game/FirstPerson/Blueprints/BP_FirstPersonCharacter.BP_FirstPersonCharacter_C|GetInventory _asbp_first_person_character))) 1))))))))
    (Development|PrintText _ip)
    (Development|PrintText (.IPaddressTarget (Utilities|Struct|BreakStruct_dataValue (Utilities|Array|Get(acopy) (Variables|/Game/BP_item/WG_inventory.WG_inventory_C|GetStruct_data (Variables|/Game/FirstPerson/Blueprints/BP_FirstPersonCharacter.BP_FirstPersonCharacter_C|GetInventory _asbp_first_person_character)) (Math|Random|RandomIntegerinRange 0 (- (Utilities|Array|Length (Variables|/Game/BP_item/WG_inventory.WG_inventory_C|GetStruct_data (Variables|/Game/FirstPerson/Blueprints/BP_FirstPersonCharacter.BP_FirstPersonCharacter_C|GetInventory _asbp_first_person_character))) 1))))))
    (if (Utilities|Enum|NotEqual(Enum) (.IPaddressTarget (Utilities|Struct|BreakStruct_dataValue (Utilities|Array|Get(acopy) (Variables|/Game/BP_item/WG_inventory.WG_inventory_C|GetStruct_data (Variables|/Game/FirstPerson/Blueprints/BP_FirstPersonCharacter.BP_FirstPersonCharacter_C|GetInventory _asbp_first_person_character)) (Math|Random|RandomIntegerinRange 0 (- (Utilities|Array|Length (Variables|/Game/BP_item/WG_inventory.WG_inventory_C|GetStruct_data (Variables|/Game/FirstPerson/Blueprints/BP_FirstPersonCharacter.BP_FirstPersonCharacter_C|GetInventory _asbp_first_person_character))) 1))))) _ip)
      (CallFunction|ShowCurrentData _output_get)
      (else
        (CallFunction|QueueWithoutDelay)))
    (else
      (Development|PrintString "wave selesai"))))

(event EventBeginPlay
  (CallFunction|QueueData))

(event Collision|EventActorBeginOverlap
  (params (OtherActor :type Actor%20Object%20Reference)))

(event EventTick
  (params (DeltaSeconds :type Float%20%28single-precision%29)))

(fn ConstructionScript)

(fn ShowCurrentData
  (params (dataID :type Integer))
  (if (>= dataID 1)
    (if (<= dataID 6)
      (Rendering|SetVisibility (Variables|Default|GetCube) true true)
      (else
        (if (== dataID 991) :!label _label
          (Rendering|SetVisibility (Variables|Default|Getvirus) true true)
          (else
            (Development|PrintString "Error ID tidak di kenal")))))
    (else
      (goto _label))))

(fn HideAllData
  (Rendering|SetVisibility (Variables|Default|GetCube) false true)
  (Rendering|SetVisibility (Variables|Default|Getvirus) false true))