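; BP_animCube is a timeline-animated cube actor that, despite its "rotate" naming, slides along the world Y axis.
; BeginPlay enables player input and plays CubeRotateTime, whose updates add RotateFloat to the current Y location, zero the rotation and print a debug string.
; The timeline restarts on finishing only while Failsafe is true; G sets the flag and Backslash clears it.
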(event EventBeginPlay
  (bind _returnvalue (Transformation|GetActorLocation))
  (Input|EnableInput (Game|GetPlayerController 0))
  (bind _rotatefloat (Timeline|cube%20rotate%20time Play)
    (:Update
      (Transformation|SetActorTransform (Math|Transform|MakeTransform (Math|Vector|MakeVector (.x _returnvalue) (+ (.y _returnvalue) (* _rotatefloat 1.0)) (.z _returnvalue)) "0.0,0.0,0.0" (Transformation|GetActorScale3D)))
      (Development|PrintString "rotate"))
    (:Finished
      (if (Variables|Default|Getfailsafe)
        (Timeline|cube%20rotate%20time PlayFromStart)))))

(event Collision|EventActorBeginOverlap
  (params (OtherActor :type Actor%20Object%20Reference)))

(event EventTick
  (params (DeltaSeconds :type Float%20%28single-precision%29)))

(event Input|KeyboardEvents|G
  (params (Key :type Key%20Structure :default "None"))
  (:Pressed
    (Variables|Default|Setfailsafe true)))

(event Input|KeyboardEvents|Backslash
  (params (Key :type Key%20Structure :default "None"))
  (:Pressed
    (Variables|Default|Setfailsafe false)))

(fn ConstructionScript)